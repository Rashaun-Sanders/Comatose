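; Actor Blueprint for a platform that shuttles back and forth between its StartPoint and EndPoint components at a set Speed.
; BeginPlay caches both points' world positions, and each Tick measures the distance travelled from the current start, then moves the actor along the normalized path direction without sweep.
; Once the travelled distance reaches the path length, start and end swap to reverse direction.
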(event `self.ReceiveBeginPlay`
  (bind _output_get (set `self.Start Location` (`SceneComponent.K2_GetComponentLocation` (`self.Start Point`))))
  (set `self.Platform Location` _output_get)
  (set `self.End Location` (`SceneComponent.K2_GetComponentLocation` (`self.EndPoint`)))
  (set `self.Speed` (`self.Speed`)))

(event `self.ReceiveTick`
  (params (DeltaSeconds :type "Float (single-precision)"))
  (`self.Set Journey Distance`)
  (bind _movedirection (`self.Set Movement Direction`))
  (bind _output_get (set `self.Platform Location` (+ (* _movedirection (* DeltaSeconds (`self.Speed`))) (`self.Platform Location`))))
  (`self.K2_SetActorLocation` _output_get))

(fn `Set Journey Distance`
  (set `self.Platform Location` (`self.K2_GetActorLocation`))
  (set `self.Path Length` (`KismetMathLibrary.VSize` (- (`self.End Location`) (`self.Start Location`))))
  (set `self.Path Travelled` (`KismetMathLibrary.VSize` (- (`self.Platform Location`) (`self.Start Location`))))
  (return))

(fn `Set Movement Direction`
  (returns (MoveDirection :type "Vector Structure"))
  (locals (MoveDirectionLocal :type "Vector Structure") (SwapLocal :type "Vector Structure"))
  (if (>= (`self.Path Travelled`) (`self.Path Length`))
    (set `local.SwapLocal` (`self.Start Location`))
    (set `self.Start Location` (`self.End Location`))
    (set `self.End Location` (`local.SwapLocal`)))
  (bind _output_get (set `local.MoveDirectionLocal` (`KismetMathLibrary.Normal` (- (`self.End Location`) (`self.Start Location`)))))
  (return _output_get))

(fn `UserConstructionScript`)