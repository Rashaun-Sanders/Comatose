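; A button-operated door that Boy_BP toggles open and closed with the Interact input while inside its trigger box.
; Box overlap enables input and opens a Gate; each press saves the boy's capsule transform as his respawn point.
; A button-press timeline nudges the mesh from its cached position, then a FlipFlop plays or reverses the door's yaw timeline.
; The door timeline's update also hides the button mesh.
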(event `InputAction|Interact`
  (params (Key :type "Key Structure"))
  (bind _button_transform_location (`KismetMathLibrary.BreakTransform` (`self.Button Transform`)))
  ;[1 1 1] E to Open
  (:`Pressed`
    (set `/Game/Blueprints/Boy_BP.RespawnLocation` (`SceneComponent.K2_GetComponentToWorld` (`Character.CapsuleComponent` (stale `self.Box.OnComponentBeginOverlap` _asboy_bp))) (stale `self.Box.OnComponentBeginOverlap` _asboy_bp))
    (`/Engine/EditorBlueprintResources/StandardMacros.Gate` true :!label _label
      (:`Exit`
        ;[1 1 1] Button
        (bind (_direction _butontrack) (`Timeline|ButtonPress` :!via `PlayFromStart`)
          (:`Update`
            (`SceneComponent.K2_SetRelativeLocation` (`self.StaticMesh`) (`KismetMathLibrary.VLerp` _button_transform_location (- _button_transform_location (0.0 5.0 0.0)) _butontrack) false false))
          (:`Finished`
            (`/Engine/EditorBlueprintResources/StandardMacros.FlipFlop`
              (:`A`
                ;[1 1 1] Open & Close Door
                (bind (_direction_2 _doortrack) (`Timeline|DoorTimeline` :!label _label_2)
                  (:`Update`
                    (`SceneComponent.K2_SetRelativeRotation` (`self.Offset`) (`KismetMathLibrary.MakeRotator` 0.0 0.0 (`KismetMathLibrary.Lerp` (`self.DoorCloseAngle`) (`self.DoorOpenAngle`) _doortrack)) false false)
                    (`SceneComponent.SetVisibility` (`self.StaticMesh`) false false))))
              (:`B`
                (goto _label_2 :!via `Reverse`)))))))))

(event `self.Box.OnComponentBeginOverlap`
  (params (OverlappedComponent :type "PrimitiveComponent Object Reference") (OtherActor :type "Actor Object Reference") (OtherComp :type "PrimitiveComponent Object Reference") (OtherBodyIndex :type Integer) (bFromSweep :type Boolean) (SweepResult :type "HitResult Structure (by ref)"))
  ;[1 1 1] E to Open
  (bind _asboy_bp (cast `/Game/Blueprints/Boy_BP` OtherActor))
  (`self.EnableInput` (`GameplayStatics.GetPlayerController` 0))
  (goto _label :!via `Open`))

(event `self.Box.OnComponentEndOverlap`
  (params (OverlappedComponent :type "PrimitiveComponent Object Reference") (OtherActor :type "Actor Object Reference") (OtherComp :type "PrimitiveComponent Object Reference") (OtherBodyIndex :type Integer))
  ;[1 1 1] E to Open
  (cast `/Game/Blueprints/Boy_BP` OtherActor)
  (`self.DisableInput` (`GameplayStatics.GetPlayerController` 0))
  (goto _label :!via `Close`))

(event `self.ReceiveBeginPlay`)

(fn `UserConstructionScript`
  (set `self.Button Transform` (`SceneComponent.GetRelativeTransform` (`self.StaticMesh`)))
  (`SceneComponent.K2_SetRelativeTransform` (`self.StaticMesh`) (`self.ButtonTransform2`) false false))